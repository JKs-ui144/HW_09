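; BP_ChatMode is a game mode running a turn-based, chat-driven number baseball game where players guess a server-generated number.
; Client messages are gated by TurnOwner, then CompareNum and ChatCheck lead to strike, ball and turn reporting.
; Messages, including non-guess chat from the turn owner, are relayed to every BP_Controller through GotBroadcast.
; A win resets the count and number; game over also flips the turn owner.
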(event `broadcast`
  ; Got BroadCast 만 분리
  (bind _outactors (`GameplayStatics.GetAllActorsOfClass` "/Script/Engine.PlayerController"))
  (for _array_element _outactors
    (bind _asbp_controller (cast `/Game/Blueprints/BP_Controller` _array_element))
    (`/Game/Blueprints/BP_Controller.GotBroadcast` _asbp_controller (`self.Player Num`))))

(event `Win`
  ; 승리시 로직
  (`KismetSystemLibrary.PrintString` (`KismetStringLibrary.Concat_StrStr` (`self.Name`) " Is Winner") true true (struct :`G` 0.66 :`B` 1.0 :`A` 1.0) 10.0)
  (`self.ResetCount And make Num`)
  (bind _outactors (`GameplayStatics.GetAllActorsOfClass` "/Script/Engine.PlayerController"))
  (for _array_element _outactors
    (bind _asbp_controller (cast `/Game/Blueprints/BP_Controller` _array_element))
    (`/Game/Blueprints/BP_Controller.GotBroadcast` _asbp_controller (`self.Player Num`))))

(event `ResetCount And make Num`
  ; 카운트 초기화 및 새로운 숫자 생성
  (`BullsAndCowsLib.resetCount` 0 0 3 (`self.BallCount`))
  (bind _returnvalue (`BullsAndCowsLib.MakeRandRange` (`self.BallCount`)))
  (bind _output_get (set `self.ServerNum` _returnvalue))
  (`KismetSystemLibrary.PrintString` (`KismetStringLibrary.Concat_StrStr` "Server make number : " _output_get) true true (struct :`G` 0.66 :`B` 1.0 :`A` 1.0) 10.0))

(event `self.ReceiveBeginPlay`
  (`BullsAndCowsLib.resetCount` 0 0 3 (`self.BallCount`))
  (bind _returnvalue (`BullsAndCowsLib.MakeRandRange` (`self.BallCount`)))
  (bind _output_get (set `self.ServerNum` _returnvalue))
  (`KismetSystemLibrary.PrintString` _output_get true true (struct :`G` 0.66 :`B` 1.0 :`A` 1.0) 10.0)
  (set `self.TurnOwner` 1))

(event `GotMessageFromClient`
  (params (Msg :type String))
  ; WhosTurn
  (set `self.Player Num` Msg)
  (bind _returnvalue (`BullsAndCowsLib.SetbIstHost` (`self.Player Num`)))
  (if (== _returnvalue (`self.TurnOwner`))
    (`self.StartGame`)
    (else
      (`KismetSystemLibrary.PrintString` "not your turn"))))

(event `StartGame`
  (bind _player_num (`self.Player Num`))
  (bind (_strikecount _ballcount _turncount) (break `BallCount` (`self.BallCount`)))
  (bind (_strikecount_2 _ballcount_2 _turncount_2) (break `BallCount` (`self.BallCount`)))
  ; 게임 로직
  (set `self.Name` (`KismetStringLibrary.Split` (`self.Player Num`) ":"))
  (`BullsAndCowsLib.CompareNum` _player_num (`self.ServerNum`) (`self.BallCount`))
  (bind _returnvalue (`BullsAndCowsLib.ChatCheck` _player_num))
  (if _returnvalue
    (`KismetSystemLibrary.PrintString` (`KismetStringLibrary.Concat_StrStr` "Strike" " : " (`KismetStringLibrary.Conv_IntToString` _strikecount_2) " " " Ball " " : " (`KismetStringLibrary.Conv_IntToString` _ballcount_2) " Turn" " : " (`KismetStringLibrary.Conv_IntToString` _turncount_2)) true true (struct :`G` 0.66 :`B` 1.0 :`A` 1.0) 10.0)
    (`|ExecutionSequence`
      (:`then_0`
        (if (>= (`.StrikeCount` (break `BallCount` (`self.BallCount`))) 3)
          (`self.Win`)
          (else
            (`self.broadcast`))))
      (:`then_1`
        (if (or (>= _ballcount 4) (<= _turncount 0))
          (`KismetSystemLibrary.PrintString` "Game Over" true true (struct :`G` 0.66 :`B` 1.0 :`A` 1.0) 10.0)
          (set `self.TurnOwner` (* (`self.TurnOwner`) -1))
          (`self.ResetCount And make Num`))))
    (else
      (`self.broadcast`))))

(fn `UserConstructionScript`)